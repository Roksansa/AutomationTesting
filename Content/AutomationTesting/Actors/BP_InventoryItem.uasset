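; BP_InventoryItem is an inventory item actor in the automation testing content that displays its type and score.
; The construction script runs Init, which picks a sphere, cube, cylinder or cone mesh from InventoryData and writes the score to a text render.
; Init applies one random color, chosen once behind IsSetColor, to a dynamic material and the text.
; On EndPlay it spawns a Niagara explosion at its location.
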(event EventEndPlay
  (params (EndPlayReason :type EEndPlayReason%20Enum :default "Destroyed"))
  (Niagara|SpawnSystematLocation "/Game/AutomationTesting/Actors/NS_Explosion.NS_Explosion" (Transformation|GetActorLocation)))

(fn ConstructionScript
  (CallFunction|Init))

(fn Init
  (bind _inventorydata (Variables|Default|GetInventoryData))
  (Components|StaticMesh|SetStaticMesh (Variables|Default|GetStaticMesh) (Utilities|Select :Index (.type _inventorydata) :SPHERE "/Engine/BasicShapes/Sphere.Sphere" :CUBE "/Engine/BasicShapes/Cube.Cube" :CYLINDER "/Engine/BasicShapes/Cylinder.Cylinder" :CONE "/Engine/BasicShapes/Cone.Cone"))
  (Rendering|Components|TextRender|SetText (Variables|Default|GetTextRender) (Utilities|Text|ToText(Integer) (.score _inventorydata)))
  (Utilities|IsValid (Variables|Init|GetMaterialInstance)
    (:Is%20Valid
      _)
    (:Is%20Not%20Valid
      (bind _returnvalue (Rendering|Material|CreateDynamicMaterialInstance (Variables|Default|GetStaticMesh) 0 "/Game/AutomationTesting/Actors/MI_InventoryItemColor.MI_InventoryItemColor" "None" :!class /Script/Engine.PrimitiveComponent))
      (Variables|Init|SetMaterialInstance _returnvalue)))
  (if (Variables|Init|GetIsSetColor)
    _
    (else
      (Variables|Init|SetIsSetColor true)
      (bind _output_get (Variables|Init|SetColor (.OutItem (Utilities|Array|Random (Variables|Init|GetLinearColorArray)))))))
  (Rendering|Material|SetMaterial (Variables|Default|GetStaticMesh) 0 (Variables|Init|GetMaterialInstance))
  (Rendering|Material|SetVectorParameterValue (Variables|Init|GetMaterialInstance) "BaseColor" _output_get :!class /Script/Engine.MaterialInstanceDynamic)
  (Rendering|Components|TextRender|SetTextRenderColor (Variables|Default|GetTextRender) (Math|Conversions|ToColor(LinearColor) (Variables|Init|GetColor))))